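; Star actor that circles the world origin at a fixed height and drives an audio tone by keypress.
; Tick sets its location from the sine and cosine of time since creation, scaled by Speed and Radius.
; BeginPlay enables input from player 0 and zeroes the Audio component's Freq parameter.
; Pressing 1 prints a debug string and raises Freq to a fixed value, with no release handling.
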(event EventBeginPlay
  (Input|EnableInput (Game|GetPlayerController 0))
  (Audio|Parameter|SetFloatParameter (Variables|Default|GetAudio) "Freq" 0.0 :!class /Script/AudioExtensions.AudioParameterControllerInterface))

(event Collision|EventActorBeginOverlap
  (params (OtherActor :type Actor%20Object%20Reference)))

(event EventTick
  (params (DeltaSeconds :type Float%20%28single-precision%29))
  (bind _returnvalue (Actor|GetGameTimeSinceCreation))
  (bind _speed (Variables|Default|GetSpeed))
  (bind _returnvalue_2 (* _returnvalue _speed))
  (Transformation|SetActorLocation (Math|Vector|MakeVector (* (Math|Trig|Sin(Degrees) _returnvalue_2) (Variables|Default|GetRadius)) (* (Math|Trig|Cos(Degrees) _returnvalue_2) (Variables|Default|GetRadius)) 1e+02) false false))

(event Input|KeyboardEvents|1
  (params (Key :type Key%20Structure :default "None"))
  (:Pressed
    (Development|PrintString "Hello")
    (Audio|Parameter|SetFloatParameter (Variables|Default|GetAudio) "Freq" 3.5e+02 :!class /Script/AudioExtensions.AudioParameterControllerInterface)))

(fn ConstructionScript)